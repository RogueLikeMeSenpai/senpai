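; Game state that keeps a reinforcement learning model's Q-table persistent between play sessions.
; On BeginPlay it loads the AI_model save slot and passes the stored table to ReinforceModel, leaving the model untouched if the cast fails.
; On EndPlay it writes the model's current Q-table into a new BP_SaveGame_AI_model object and saves it to that slot.
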(event EventBeginPlay
  (bind _returnvalue (SaveGame|LoadGamefromSlot "AI_model"))
  (bind _asbp_save_game_ai_model (Utilities|Casting|CastToBP_SaveGame_AI_model _returnvalue))
  (Class|ReinforceModel|SetQtable (Variables|Default|GetReinforceModel) (Variables|/Game/Developers/pschl/BP_SaveGame_AI_model.BP_SaveGame_AI_model_C|GetQ_table _asbp_save_game_ai_model)))

(event EventTick
  (params (DeltaSeconds :type Float%20%28single-precision%29)))

(event EventEndPlay
  (params (EndPlayReason :type EEndPlayReason%20Enum :default "Destroyed"))
  (bind _returnvalue (SaveGame|CreateSaveGameObject "/Game/Developers/pschl/BP_SaveGame_AI_model.BP_SaveGame_AI_model_C"))
  (Variables|/Game/Developers/pschl/BP_SaveGame_AI_model.BP_SaveGame_AI_model_C|SetQ_table _returnvalue (Class|ReinforceModel|GetQtable (Variables|Default|GetReinforceModel)))
  (SaveGame|SaveGametoSlot _returnvalue "AI_model"))

(fn ConstructionScript)