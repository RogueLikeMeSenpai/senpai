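; Game mode for SenpAI that handles level progression, player spawn selection and restarts after death.
; Each new player triggers level registration and a tracking event on the game instance, using values parsed from the URL options string.
; Spawning prefers a Play-From-Here start, then the checkpoint option, then the default start.
; Death reloads the current level when a checkpoint exists, otherwise returns to level 1, or 0 from the first.
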(event EventBeginPlay
  (bind _assenpai_game_instance_base (Utilities|Casting|CastToSenpaiGameInstanceBase (Game|GetGameInstance)))
  (Variables|Default|SetgameInstance _assenpai_game_instance_base))

(event EventHandleStartingNewPlayer
  (params (NewPlayer :type Player%20Controller%20Object%20Reference))
  (CallFunction|RegisterLevelChange)
  (CallFunction|ChooseStart NewPlayer))

(fn ConstructionScript)

(fn RegisterLevelChange
  ;[1 1 1] Ensure Game Instance is set
  (Utilities|IsValid (Variables|Default|GetgameInstance)
    (:Is%20Valid
      _)
    (:Is%20Not%20Valid
      (bind _assenpai_game_instance_base (Utilities|Casting|CastToSenpaiGameInstanceBase (Game|GetGameInstance)))
      (Variables|Default|SetgameInstance _assenpai_game_instance_base)))
  ;[1 1 1] Register Level Change
  (Class|SenpaiGameInstanceBase|RegisterLevelChange (Variables|Default|GetgameInstance) (Class|GameplayStatics|GetIntOption (Variables|Default|GetOptionsString) "level") (Math|Conversions|ToBoolean(Integer) (Class|GameplayStatics|GetIntOption (Variables|Default|GetOptionsString) "death")))
  (Class|SenpaiGameInstanceBase|Track (Variables|Default|GetgameInstance) "level_start" (LocalVariables|GetemptyMap))
  ;[1 1 1] Debug Output
  (Development|PrintString (Utilities|String|ToString(Text) (Utilities|Text|FormatText "CurrentRun={CurrentRun}; CurrentLevel={CurrentLevel}" (Variables|/Script/senpai.SenpaiGameInstanceBase|GetCurrentRun (Variables|Default|GetgameInstance)) (Variables|/Script/senpai.SenpaiGameInstanceBase|GetCurrentLevel (Variables|Default|GetgameInstance)))) true true "(R=0.000000,G=0.660000,B=1.000000,A=1.000000)" 1e+01))

(fn ChooseStart
  (params (playerController :type Player%20Controller%20Object%20Reference))
  (bind _outactors (Actor|GetAllActorsOfClass "/Script/Engine.PlayerStartPIE"))
  (if (Utilities|Array|IsNotEmpty _outactors)
    (Class|GameModeBase|RestartPlayeratPlayerStart playerController (Utilities|Array|Get(acopy) _outactors))
    (else
      (bind _output_get (LocalVariables|Setcheckpoint (Class|GameplayStatics|ParseOption (Variables|Default|GetOptionsString) "checkpoint")))
      (if (Utilities|Array|IsEmpty _output_get)
        ;[1 1 1] Start from Default
        (Class|GameModeBase|RestartPlayeratPlayerStart playerController (Class|GameModeBase|FindPlayerStart playerController "None"))
        (else
          ;[1 1 1] Start From Checkpoint
          (Class|GameModeBase|RestartPlayeratPlayerStart playerController (Class|GameModeBase|FindPlayerStart playerController (LocalVariables|Getcheckpoint))))))))

(fn NextLevel
  (bind _gameinstance (Variables|Default|GetgameInstance))
  (bind _currentlevel (Variables|/Script/senpai.SenpaiGameInstanceBase|GetCurrentLevel _gameinstance))
  (bind _returnvalue (+ _currentlevel 1))
  (Game|OpenLevel(byObjectReference) (Utilities|Array|Get(acopy) (Variables|Default|GetLevels) _returnvalue) true (Utilities|String|Append "level=" (Utilities|String|ToString(Integer) _returnvalue))))

(fn ChangeLevelonDeath
  (if (Utilities|Array|IsEmpty (Variables|/Script/senpai.SenpaiGameInstanceBase|Getcheckpoint (Variables|Default|GetgameInstance)))
    (if (> (Variables|/Script/senpai.SenpaiGameInstanceBase|GetCurrentLevel (Variables|Default|GetgameInstance)) 0)
      ;[1 1 1] Back to Level 1
      (Game|OpenLevel(byObjectReference) (Utilities|Array|Get(acopy) (Variables|Default|GetLevels) 1) true (Utilities|MakeOptions true 1 (Variables|/Script/senpai.SenpaiGameInstanceBase|Getcheckpoint (Variables|Default|GetgameInstance))))
      (else
        ;[1 1 1] Back to Level 0
        (Game|OpenLevel(byObjectReference) (Utilities|Array|Get(acopy) (Variables|Default|GetLevels)) true (Utilities|MakeOptions true 0 (Variables|/Script/senpai.SenpaiGameInstanceBase|Getcheckpoint (Variables|Default|GetgameInstance))))))
    (else
      ;[1 1 1] Restart current Level
      (bind _returnvalue (Game|GetCurrentLevelName true))
      (Game|OpenLevel(byName) (Utilities|String|StringToName _returnvalue) true (Utilities|MakeOptions true (Variables|/Script/senpai.SenpaiGameInstanceBase|GetCurrentLevel (Variables|Default|GetgameInstance)) (Variables|/Script/senpai.SenpaiGameInstanceBase|Getcheckpoint (Variables|Default|GetgameInstance)))))))