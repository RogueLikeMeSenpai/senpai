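; Trigger actor that plays a one-shot cinematic camera tour when the player character overlaps it.
; If no targets are set, it gathers every BP_SimpleEnemy_Character, retrying on a delay until some exist.
; A recursive event with delays blends the view target through each target in cinematic mode.
; On an invalid index or target, it blends back to the player and ends cinematic mode.
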(event Custom|MoveCam
  (params (index :type Integer))
  ;[1 1 1] Move from target to target and back to player
  (bind (_delay _finished _nextindex) (CallFunction|MoveView index 0.5 0.75))
  (Utilities|FlowControl|Delay _delay)
  (if _finished
    (Class|PlayerController|SetCinematicMode (Game|GetPlayerController 0) false false true true false)
    (else
      (CallFunction|MoveCam _nextindex))))

(event Custom|Start%20Dolly%20Shot
  ;[1 1 1] Start the dolly shot
  (if (Variables|Default|Getenabled)
    (Variables|Default|Setenabled false)
    (if (Utilities|Array|IsNotEmpty (Variables|Default|Gettargets))
      (CallFunction|MoveCam)
      (else
        (bind _targets (CallFunction|InitTargets :!label _label))
        (if (Utilities|Array|IsNotEmpty _targets)
          (CallFunction|MoveCam)
          (else
            (Utilities|FlowControl|Delay 0.5)
            (goto _label)))))))

(event EventBeginPlay)

(event Collision|EventActorBeginOverlap
  (params (OtherActor :type Actor%20Object%20Reference))
  (if (== OtherActor (Game|GetPlayerCharacter 0))
    (CallFunction|StartDollyShot)))

(event EventTick
  (params (DeltaSeconds :type Float%20%28single-precision%29)))

(fn ConstructionScript)

(fn MoveView
  (params (index :type Integer) (blendTime :type Float%20%28double-precision%29) (stayTime :type Float%20%28double-precision%29))
  (bind _targets (Variables|Default|Gettargets))
  (bind _output (Utilities|Array|Get(acopy) _targets index))
  (LocalVariables|Settarget _output)
  (Utilities|IsValid _output
    (:Is%20Valid
      (Class|PlayerController|SetCinematicMode (Game|GetPlayerController 0) true false true true false)
      (Game|Player|SetViewTargetwithBlend (Game|GetPlayerController 0) (LocalVariables|Gettarget) blendTime "VTBlend_Linear" 0.0 true)
      (bind _result (Math|Integer|IncrementInt index)
        (:%20%20
          (return (+ blendTime stayTime) false _result))))
    (:Is%20Not%20Valid
      (Game|Player|SetViewTargetwithBlend (Game|GetPlayerController 0) (Game|GetPlayerCharacter 0) 1.0 "VTBlend_Linear" 0.0 false)
      (return 0.0 true 0))))

(fn InitTargets
  (bind _outactors (Actor|GetAllActorsOfClass "/Game/SenpAI/Core/Characters/BP_SimpleEnemy_Character.BP_SimpleEnemy_Character_C"))
  (bind _output_get (Variables|Default|Settargets _outactors))
  (return _output_get))