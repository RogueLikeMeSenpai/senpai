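; BP_EnemyEntrance is an enemy spawn point that creates and configures an AI enemy from a given EnemyConfig.
; Its Spawn event spawns the configured pawn class at SpawnLocation running BT_SimpleEnemy, then passes the config Id to the AI controller as its model tags.
; The attack behavior is injected as a dynamic subtree under the EngagedBehavior tag, and the spawned weapon's events are bound to the controller.
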(event Custom|Spawn
  (params (EnemyConfig :type Structure%20Enemy%20Config%20Structure))
  (CallFunction|SpawnEnemy EnemyConfig))

(fn ConstructionScript)

(fn SpawnEnemy
  (params (EnemyConfig :type Structure%20Enemy%20Config%20Structure))
  (bind _returnvalue (AI|SpawnAIFromClass (.characterclass EnemyConfig) "/Game/SenpAI/Core/AI/BT_SimpleEnemy.BT_SimpleEnemy" (Transformation|GetWorldLocation (Variables|Default|GetSpawnLocation)) "0, 0, 0" false 0))
  (bind _asbp_simple_enemy_character (Utilities|Casting|CastToBP_SimpleEnemy_Character _returnvalue))
  (bind _output_get (LocalVariables|SetEnemy _asbp_simple_enemy_character))
  (bind _asaic_simple_enemy (Utilities|Casting|CastToAIC_SimpleEnemy (AI|GetAIController _output_get)))
  (bind _output_get_2 (LocalVariables|SetAIC _asaic_simple_enemy))
  (Variables|/Game/SenpAI/Core/AI/AIC_SimpleEnemy.AIC_SimpleEnemy_C|SetModelTagsStr _output_get_2 (.id EnemyConfig))
  (Utilities|FlowControl|Sequence
    (:then_0
      ;[1 1 1] Attack Behavior
      (bind _asbehavior_tree_component (Utilities|Casting|CastToBehaviorTreeComponent (Variables|/Script/AIModule.AIController|GetBrainComponent (LocalVariables|GetAIC))))
      (Class|BehaviorTreeComponent|SetDynamicSubtree _asbehavior_tree_component "(TagName=\"EngagedBehavior\")" (.attackbehavior EnemyConfig)))
    (:then_1
      ;[1 1 1] Weapon
      (bind _weapon (Default|SpawnWeapon (LocalVariables|GetEnemy) (.weaponclass EnemyConfig)))
      (Default|BindWeaponEvents (LocalVariables|GetAIC) _weapon))))