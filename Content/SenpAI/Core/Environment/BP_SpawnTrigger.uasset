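; BP_SpawnTrigger is a one-shot box trigger that spawns enemies through color-matched entrance actors when overlapped.
; On BeginPlay it maps spawn entrances by color, gets the enemy config from the game mode, and stays disabled until the game state's AI model loads.
; On overlap it spawns the static list if filled, otherwise asks the reinforcement model to create the set amount of enemies.
; Each config ID resolves to a config whose color selects the entrance.
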(event OnComponentBeginOverlap(Box)
  (params (OverlappedComponent :type Primitive%20Component%20Object%20Reference) (OtherActor :type Actor%20Object%20Reference) (OtherComp :type Primitive%20Component%20Object%20Reference) (OtherBodyIndex :type Integer) (bFromSweep :type Boolean) (SweepResult :type Hit%20Result%20Structure%20%28by%20ref%29))
  ;[1 1 1] Overlap Trigger
  (if (Variables|Default|GetEnabled)
    (Variables|Default|SetEnabled false)
    (if (Utilities|Array|IsEmpty (Variables|Default|GetStaticSpawnList))
      ;[1 1 1] Spawn From AI Model
      (for _index (range 1 (Variables|Default|GetAmount))
        (bind _returnvalue (Class|AImodel|CreateEnemy (Variables|Default|GetAIModel)))
        (CallFunction|Spawn _returnvalue))
      (else
        ;[1 1 1] Spawn Static
        (for _array_element (Variables|Default|GetStaticSpawnList)
          (CallFunction|Spawn _array_element))))))

(event Custom|OnAIModelLoaded
  (params (AIModel :type A%20Imodel%20Object%20Reference))
  ;[1 1 1] Enable On AI Model Loaded
  (Variables|Default|SetAIModel AIModel)
  (Variables|Default|SetEnabled true))

(event Custom|Spawn
  (params (EnemyConfigId :type String))
  ;[1 1 1] Spawn
  (bind _enemyconfig1 (Default|GetEnemyConfig (Variables|Default|GetEnemy%20Config) EnemyConfigId))
  (Default|Spawn (.Value (Utilities|Map|Find (Variables|Default|GetEntrances) (.Color (Utilities|Struct|BreakStructure_EnemyConfig _enemyconfig1)))) _enemyconfig1))

(event EventBeginPlay
  ;[1 1 1] Init
  (Utilities|FlowControl|Sequence
    (:then_0
      ;[1 1 1] Get Entrances
      (bind _outactors (Actor|GetAllActorsOfClass "/Game/SenpAI/Core/Environment/BP_EnemySpawnEntrance.BP_EnemySpawnEntrance_C"))
      (for _array_element _outactors
        (Utilities|Map|Add (Variables|Default|GetEntrances) (Variables|/Game/SenpAI/Core/Environment/BP_EnemySpawnEntrance.BP_EnemySpawnEntrance_C|GetEnemyColor _array_element) _array_element)))
    (:then_1
      ;[1 1 1] Get Enemy Configs
      (bind _asbp_senpai_game_mode (Utilities|Casting|CastToBP_Senpai_GameMode (Game|GetGameMode)))
      (Variables|Default|SetEnemy%20Config (Variables|/Game/SenpAI/Core/GameModes/BP_Senpai_GameMode.BP_Senpai_GameMode_C|GetEnemyConfig _asbp_senpai_game_mode)))
    (:then_2
      ;[1 1 1] Get AI Model
      (bind _asbp_game_state_reinforcment_model (Utilities|Casting|CastToBP_GameState_ReinforcmentModel (Game|GetGameState)))
      (EventDispatchers|BindEventtoLoadedAIModel _asbp_game_state_reinforcment_model (delegate Custom|OnAIModelLoaded)))))

(fn ConstructionScript)