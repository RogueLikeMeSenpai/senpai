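; BP_EnemySpawnEntrance is a color-coded fog gate that spawns enemies from an EnemyConfig, with its fog material set at construction.
; SpawnEnemy creates the pawn on a shared behavior tree, passes on the gate's Lock and color, and injects the config's attack behavior as a dynamic subtree.
; It binds the weapon, tracks the spawn through the GameInstance, and sends the enemy toward a random point near PresentationLocation.
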(event Custom|Spawn
  (params (EnemyConfig :type BP%20Single%20Enemy%20Config%20Asset%20Object%20Reference))
  (CallFunction|SpawnEnemy EnemyConfig))

(event EventBeginPlay
  (bind _assenpai_game_instance_base (Utilities|Casting|CastToSenpaiGameInstanceBase (Game|GetGameInstance)))
  (Variables|Default|SetGameInstance _assenpai_game_instance_base))

(fn ConstructionScript
  (switch Utilities|FlowControl|Switch|SwitchonEnum_EnemyColor (Variables|Default|GetEnemyColor)
    (:NewEnumerator0
      (Rendering|Material|SetMaterial (Variables|Default|GetFogGate) 0 "/Game/SenpAI/Materials/M_SpawnGateFog_Green.M_SpawnGateFog_Green"))
    (:NewEnumerator1
      (Rendering|Material|SetMaterial (Variables|Default|GetFogGate) 0 "/Game/SenpAI/Materials/M_SpawnGateFog_Blue.M_SpawnGateFog_Blue"))
    (:NewEnumerator2
      (Rendering|Material|SetMaterial (Variables|Default|GetFogGate) 0 "/Game/SenpAI/Materials/M_SpawnGateFog_Red.M_SpawnGateFog_Red"))))

(fn SpawnEnemy
  (params (EnemyConfig :type BP%20Single%20Enemy%20Config%20Asset%20Object%20Reference))
  (bind _returnvalue (AI|SpawnAIFromClass (Variables|/Game/SenpAI/Core/AI/EnemyConfig/BP_SingleEnemyConfig_Asset.BP_SingleEnemyConfig_Asset_C|GetCharacterClass EnemyConfig) "/Game/SenpAI/Core/AI/BT_SimpleEnemy.BT_SimpleEnemy" (Transformation|GetWorldLocation (Variables|Default|GetSpawnLocation)) "0, 0, 0" false 0))
  (bind _asbp_simple_enemy_character (Utilities|Casting|CastToBP_SimpleEnemy_Character _returnvalue))
  (bind _output_get (LocalVariables|SetEnemy _asbp_simple_enemy_character))
  (Variables|/Game/SenpAI/Core/Characters/BP_SimpleEnemy_Character.BP_SimpleEnemy_Character_C|Setlock _output_get (Variables|Default|Getlock))
  (bind _asaic_simple_enemy (Utilities|Casting|CastToAIC_SimpleEnemy (AI|GetAIController _output_get)))
  (bind _output_get_2 (LocalVariables|SetAIC _asaic_simple_enemy))
  (Variables|/Game/SenpAI/Core/AI/AIC_SimpleEnemy.AIC_SimpleEnemy_C|SetModelTagsStr _output_get_2 (Variables|/Game/SenpAI/Core/AI/EnemyConfig/BP_SingleEnemyConfig_Asset.BP_SingleEnemyConfig_Asset_C|GetId EnemyConfig))
  (Utilities|FlowControl|Sequence
    (:then_0
      ;[1 1 1] Track
      (Class|SenpaiGameInstanceBase|Track (Variables|Default|GetGameInstance) "enemy_spawn" (Utilities|Map|MakeMap "enemy_type" (Variables|/Game/SenpAI/Core/AI/EnemyConfig/BP_SingleEnemyConfig_Asset.BP_SingleEnemyConfig_Asset_C|GetId EnemyConfig) "room_name" (Variables|Default|GetRoomName))))
    (:then_1
      ;[1 1 1] Attack Behavior
      (bind _asbehavior_tree_component (Utilities|Casting|CastToBehaviorTreeComponent (Variables|/Script/AIModule.AIController|GetBrainComponent (LocalVariables|GetAIC))))
      (Class|BehaviorTreeComponent|SetDynamicSubtree _asbehavior_tree_component "(TagName=\"EngagedBehavior\")" (Variables|/Game/SenpAI/Core/AI/EnemyConfig/BP_SingleEnemyConfig_Asset.BP_SingleEnemyConfig_Asset_C|GetAttackBehavior EnemyConfig)))
    (:then_2
      ;[1 1 1] Weapon
      (bind _weapon (Default|SpawnWeapon (LocalVariables|GetEnemy) (Variables|/Game/SenpAI/Core/AI/EnemyConfig/BP_SingleEnemyConfig_Asset.BP_SingleEnemyConfig_Asset_C|GetWeaponClass EnemyConfig)))
      (Default|BindWeaponEvents (LocalVariables|GetAIC) _weapon))
    (:then_3
      ;[1 1 1] Color
      (Default|ChangeColor (LocalVariables|GetEnemy) (Variables|Default|GetEnemyColor)))
    (:then_4
      ;[1 1 1] Presentation
      (Variables|/Game/SenpAI/Core/AI/AIC_SimpleEnemy.AIC_SimpleEnemy_C|SetremarkAnim (LocalVariables|GetAIC) (Variables|/Game/SenpAI/Core/AI/EnemyConfig/BP_SingleEnemyConfig_Asset.BP_SingleEnemyConfig_Asset_C|GetRemarkAnim EnemyConfig))
      (Default|ChangeState (LocalVariables|GetAIC) "NewEnumerator3")
      (AI|Components|Blackboard|SetValueasVector (AI|GetBlackboard (LocalVariables|GetAIC)) (Utilities|Name|MakeLiteralName "TargetLocation") (.RandomLocation (AI|Navigation|GetRandomReachablePointinRadius (Transformation|GetWorldLocation (Variables|Default|GetPresentationLocation)) 2e+02 0 0))))
    (:then_5
      ;[1 1 1] Return
      (return (LocalVariables|GetAIC)))))