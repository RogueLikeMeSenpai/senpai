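; BP_SpikeTrap is an environmental hazard that deals lethal-scale damage to any actor overlapping its Box_Death volume.
; A second volume, Box_Edge, serves as an edge warning for simple enemies by notifying their AIC_SimpleEnemy controller.
; On overlap it calls BeginOnEdge with the sweep's location and normal, and on exit it calls EndOnEdge.
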(event OnComponentBeginOverlap(Box_Death)
  (params (OverlappedComponent :type Primitive%20Component%20Object%20Reference) (OtherActor :type Actor%20Object%20Reference) (OtherComp :type Primitive%20Component%20Object%20Reference) (OtherBodyIndex :type Integer) (bFromSweep :type Boolean) (SweepResult :type Hit%20Result%20Structure%20%28by%20ref%29))
  (Game|Damage|ApplyDamage OtherActor 1e+04 0 self))

(event OnComponentBeginOverlap(Box_Edge)
  (params (OverlappedComponent :type Primitive%20Component%20Object%20Reference) (OtherActor :type Actor%20Object%20Reference) (OtherComp :type Primitive%20Component%20Object%20Reference) (OtherBodyIndex :type Integer) (bFromSweep :type Boolean) (SweepResult :type Hit%20Result%20Structure%20%28by%20ref%29))
  (bind (_bblockinghit _binitialoverlap _time _distance _location _impactpoint _normal) (Collision|BreakHitResult SweepResult))
  (bind _asbp_simple_enemy_character (Utilities|Casting|CastToBP_SimpleEnemy_Character OtherActor))
  (bind _asaic_simple_enemy (Utilities|Casting|CastToAIC_SimpleEnemy (Pawn|GetController _asbp_simple_enemy_character)))
  (Default|BeginonEdge _asaic_simple_enemy _location _normal))

(event OnComponentEndOverlap(Box_Edge)
  (params (OverlappedComponent :type Primitive%20Component%20Object%20Reference) (OtherActor :type Actor%20Object%20Reference) (OtherComp :type Primitive%20Component%20Object%20Reference) (OtherBodyIndex :type Integer))
  (bind _asbp_simple_enemy_character (Utilities|Casting|CastToBP_SimpleEnemy_Character OtherActor))
  (bind _asaic_simple_enemy (Utilities|Casting|CastToAIC_SimpleEnemy (Pawn|GetController _asbp_simple_enemy_character)))
  (Default|EndonEdge _asaic_simple_enemy))

(event EventBeginPlay)

(event Collision|EventActorBeginOverlap
  (params (OtherActor :type Actor%20Object%20Reference)))

(event EventTick
  (params (DeltaSeconds :type Float%20%28single-precision%29)))

(fn ConstructionScript)