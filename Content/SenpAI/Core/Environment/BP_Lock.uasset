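; BP_Lock is a soul-counting lock that opens a door once enough BP_Soul actors overlap it.
; A preset soul count builds its stack of segment meshes in the construction script; otherwise BeginPlay sums the amounts from selected, or all, spawn triggers and builds it then.
; Each soul switches a segment to the unlocked material with a click sound, and the final one opens the assigned door or the first one found.
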(event EventBeginPlay
  (if (<= (Variables|Default|GetrequiredSouls) 0)
    (if (Utilities|Array|IsEmpty (Variables|Default|GetspawnTrigger))
      ;[1 1 1] Init Segments from all spawn triggers
      (Variables|Default|SetrequiredSouls 0)
      (bind _outactors (Actor|GetAllActorsOfClass "/Game/SenpAI/Core/Environment/BP_SpawnTrigger.BP_SpawnTrigger_C"))
      (for _array_element _outactors
        (Variables|Default|SetrequiredSouls (+ (Variables|Default|GetrequiredSouls) (Variables|/Game/SenpAI/Core/Environment/BP_SpawnTrigger.BP_SpawnTrigger_C|GetAmount _array_element))))
      (CallFunction|InitializeSegments)
      (else
        ;[1 1 1] Init Segments from selected spawn triggers
        (Variables|Default|SetrequiredSouls 0)
        (for _array_element_2 (Variables|Default|GetspawnTrigger)
          (Variables|Default|SetrequiredSouls (+ (Variables|Default|GetrequiredSouls) (Variables|/Game/SenpAI/Core/Environment/BP_SpawnTrigger.BP_SpawnTrigger_C|GetAmount _array_element_2))))
        (CallFunction|InitializeSegments)))))

(event Collision|EventActorBeginOverlap
  (params (OtherActor :type Actor%20Object%20Reference))
  (if (== (Utilities|GetClass OtherActor) "/Game/SenpAI/Core/Environment/BP_Soul.BP_Soul_C")
    (CallFunction|UnlockSegment)
    (Audio|PlaySoundatLocation "/Game/SenpAI/Audio/Sounds/Environment/A_Lever_click_Cue.A_Lever_click_Cue" (Transformation|GetActorLocation) "0, 0, 0" 1.0 1.0 0.0 0 0 0 0)))

(fn ConstructionScript
  (if (> (Variables|Default|GetrequiredSouls) 0)
    (CallFunction|InitializeSegments)))

(fn UnlockSegment
  (bind _door (Variables|Default|Getdoor))
  (Utilities|IsValid (Utilities|Array|Get(acopy) (Variables|Default|GetlockSegments) (Variables|Default|GetsoulsCount))
    (:Is%20Valid
      (Rendering|Material|SetMaterial (Utilities|Array|Get(acopy) (Variables|Default|GetlockSegments) (Variables|Default|GetsoulsCount)) 1 "/Game/SenpAI/Art/Lock/M_Lock_Segment_Unlocked.M_Lock_Segment_Unlocked"))
    (:Is%20Not%20Valid
      _))
  (bind _result (Math|Integer|IncrementInt (Variables|Default|GetsoulsCount))
    (:%20%20
      (bind _output_get (Variables|Default|SetsoulsCount _result))
      (if (and (>= _output_get (Variables|Default|GetrequiredSouls)) (not (Variables|Default|Getunlocked)))
        ;[1 1 1] Open Door
        (if (Utilities|IsValid _door)
          (Default|Open _door)
          (else
            (bind _outactors (Actor|GetAllActorsOfClass "/Game/SenpAI/Core/Environment/BP_Door.BP_Door_C"))
            (Default|Open (Utilities|Array|Get(acopy) _outactors))))
        (Variables|Default|Setunlocked true)))))

(fn InitializeSegments
  (Components|DestroyComponent (Variables|Default|GetTemporarySegment))
  ;[1 1 1] Add Lock Segments
  (for _index (range 0 (- (Variables|Default|GetrequiredSouls) 1))
    ;;[1 1 1] Use Instanced?
    (bind _returnvalue (AddComponent|AddStaticMeshComponent false (LocalVariables|GetRelative%20Transform)))
    (Utilities|Array|Add (Variables|Default|GetlockSegments) _returnvalue)
    (Components|StaticMesh|SetStaticMesh _returnvalue "/Game/SenpAI/Art/Lock/S_Lock_Segment.S_Lock_Segment")
    ;[1 1 1] Calculate new Transform for offset
    (LocalVariables|SetRelative%20Transform (Math|Transform|MakeTransform (Math|Vector|MakeVector (.x (.location (LocalVariables|GetRelative%20Transform))) (.y (.location (LocalVariables|GetRelative%20Transform))) (+ (.z (.location (LocalVariables|GetRelative%20Transform))) (.z (.Max (Components|StaticMesh|GetLocalBounds _returnvalue))))) (.rotation (LocalVariables|GetRelative%20Transform)) (.scale (LocalVariables|GetRelative%20Transform))))))