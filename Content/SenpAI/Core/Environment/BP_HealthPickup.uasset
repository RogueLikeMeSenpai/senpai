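; BP_HealthPickup is a health pickup actor that bobs in place and heals whatever actor overlaps it.
; A Hovering timeline drives the sphere's relative Z, starting at a random time so instances bob out of sync.
; Overlap applies negative damage without filtering the actor, plays a pickup sound, destroys the pickup and prints a message.
; GetNearestLock and an empty MoveTowardsDestination are present but never called here.
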(event EventBeginPlay
  ;[1 1 1] Hovering
  (Utilities|FlowControl|Sequence
    (:then_0
      (bind _height (Timeline|Hovering SetNewTime)
        (:Update
          (Transformation|SetRelativeLocation (Variables|Default|GetSphere) (Math|Vector|MakeVector 0.0 0.0 (* _height (Variables|Default|GetHoverRelativeDistance))) false false))))
    (:then_1
      (Timeline|Hovering Play))))

(event Collision|EventActorBeginOverlap
  (params (OtherActor :type Actor%20Object%20Reference))
  ;[1 1 1] Pickup
  (Game|Damage|ApplyDamage OtherActor (* (Variables|Default|GetHealAmount) -1.0) 0 self)
  (Audio|PlaySound2D "/Game/SenpAI/Audio/Sounds/Environment/A_Orb_pickup_Cue.A_Orb_pickup_Cue" 1.0 1.0 0.0 0 0)
  (Actor|DestroyActor)
  (Development|PrintString "Healed"))

(fn ConstructionScript)

(fn MoveTowardsDestination
  (params (DeltaTime :type Float%20%28single-precision%29)))

(fn GetNearestLock
  (bind _outactors (Actor|GetAllActorsOfClass "/Game/SenpAI/Core/Environment/BP_Lock.BP_Lock_C"))
  (LocalVariables|SetnearestLock (Utilities|Array|Get(acopy) _outactors))
  (LocalVariables|SetnearestDistance (Transformation|GetDistanceTo (Utilities|Array|Get(acopy) _outactors) self))
  (for _array_element _outactors
    (if (< (Transformation|GetDistanceTo _array_element self) (LocalVariables|GetnearestDistance))
      (LocalVariables|SetnearestDistance (Transformation|GetDistanceTo _array_element self))
      (LocalVariables|SetnearestLock _array_element)))
  (return (LocalVariables|GetnearestLock)))