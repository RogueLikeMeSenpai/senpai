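; BP_Soul is a collectible orb that hovers until the player character overlaps it, then flies to a lock.
; A Hovering timeline bobs the sphere mesh from a random start time, so souls move out of phase.
; Pickup plays a sound and targets a point above the first BP_Lock found in the level.
; Tick moves it there at constant speed and destroys it on arrival, while MoveTowardsDestination is an empty stub.
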(event EventBeginPlay
  (Utilities|FlowControl|Sequence
    (:then_0
      (bind _height (Timeline|Hovering SetNewTime)
        (:Update
          (Transformation|SetRelativeLocation (Variables|Default|GetSphere) (Math|Vector|MakeVector 0.0 0.0 (* _height (Variables|Default|GetHoverRelativeDistance))) false false))))
    (:then_1
      (Timeline|Hovering Play))))

(event Collision|EventActorBeginOverlap
  (params (OtherActor :type Actor%20Object%20Reference))
  (if (and (not (Variables|Default|GetCollected)) (== OtherActor (Game|GetPlayerCharacter 0)))
    ;[1 1 1] TODO do somewhere else
    (bind _outactors (Actor|GetAllActorsOfClass "/Game/SenpAI/Core/Environment/BP_Lock.BP_Lock_C"))
    (Variables|Default|SetDestination (+ (Transformation|GetActorLocation (Utilities|Array|Get(acopy) _outactors)) "0,0,100.000000"))
    (Variables|Default|SetCollected true)
    (Audio|PlaySound2D "/Game/SenpAI/Audio/Sounds/Environment/A_Orb_pickup_Cue.A_Orb_pickup_Cue" 1.0 1.0 0.0 0 0)))

(event EventTick
  (params (DeltaSeconds :type Float%20%28single-precision%29))
  (if (Variables|Default|GetCollected)
    ;[1 1 1] Move towards Destination
    (Transformation|SetActorLocation (Math|Interpolation|VInterptoConstant (Transformation|GetActorLocation) (Variables|Default|GetDestination) DeltaSeconds 6e+02) false false)
    (if (<= (Math|Vector|Distance(Vector) (Transformation|GetActorLocation) (Variables|Default|GetDestination)) 1.0)
      (Actor|DestroyActor))))

(fn ConstructionScript)

(fn MoveTowardsDestination
  (params (DeltaTime :type Float%20%28single-precision%29)))