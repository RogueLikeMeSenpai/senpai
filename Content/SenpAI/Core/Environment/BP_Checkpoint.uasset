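; BP_Checkpoint is a trigger volume that records the player's progress as a checkpoint in the game instance.
; When something overlaps its box while enabled, it disables itself, then, if the overlapper is the player character, stores its PlayerStart tag as the current checkpoint and prints it.
; The disable happens before the player check, so any first overlapping actor uses up the checkpoint.
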(event OnComponentBeginOverlap(Box)
  (params (OverlappedComponent :type Primitive%20Component%20Object%20Reference) (OtherActor :type Actor%20Object%20Reference) (OtherComp :type Primitive%20Component%20Object%20Reference) (OtherBodyIndex :type Integer) (bFromSweep :type Boolean) (SweepResult :type Hit%20Result%20Structure%20%28by%20ref%29))
  (if (Variables|Default|Getenabled)
    (Variables|Default|Setenabled false)
    (Utilities|Casting|CastToBP_PlayerCharacter OtherActor)
    (bind _output_get (Variables|/Script/senpai.SenpaiGameInstanceBase|Setcheckpoint (Variables|Default|GetgameInstance) (Utilities|String|ToString(Name) (Variables|Default|GetplayerStartTag))))
    (Development|PrintString (Utilities|String|Append "Checkpoint=" _output_get))))

(event EventBeginPlay
  (bind _assenpai_game_instance_base (Utilities|Casting|CastToSenpaiGameInstanceBase (Game|GetGameInstance)))
  (Variables|Default|SetgameInstance _assenpai_game_instance_base))

(event Collision|EventActorBeginOverlap
  (params (OtherActor :type Actor%20Object%20Reference)))

(event EventTick
  (params (DeltaSeconds :type Float%20%28single-precision%29)))

(fn ConstructionScript)