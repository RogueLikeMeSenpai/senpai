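; Enemy spawn point that spawns a configurable AI pawn with the simple-enemy behavior tree shortly after BeginPlay.
; It tags the pawn's AI controller from its TagString, or from a config generated by the game state's reinforcement model when TagString is empty.
; It then registers its name and the chosen enemy config with the game instance.
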(event Custom|AllSpawnPointsReady)

(event EventBeginPlay
  (Utilities|FlowControl|Delay 0.5)
  (bind _returnvalue (AI|SpawnAIFromClass (Variables|Default|GetClass%20To%20Spawn) "/Game/SenpAI/Core/AI/BT_SimpleEnemy.BT_SimpleEnemy" (Transformation|GetActorLocation) "0, 0, 0" false 0))
  (CallFunction|ApplyTags _returnvalue)
  (bind _asgame_instance_alex (Utilities|Casting|CastToGameInstanceAlex (Game|GetGameInstance)))
  (Default|AddSpawn _asgame_instance_alex (Utilities|GetObjectName self) (Variables|Default|GetEnemyConfig)))

(event EventTick
  (params (DeltaSeconds :type Float%20%28single-precision%29)))

(fn ConstructionScript)

(fn ApplyTags
  (params (SpawnedPawn :type Pawn%20Object%20Reference))
  (bind _asaic_simple_enemy (Utilities|Casting|CastToAIC_SimpleEnemy (AI|GetAIController SpawnedPawn)))
  (LocalVariables|SetAIController _asaic_simple_enemy)
  (bind _asbp_game_state_reinforcment_model (Utilities|Casting|CastToBP_GameState_ReinforcmentModel (Game|GetGameState)))
  (LocalVariables|SetReinforcmentModel (Variables|/Game/SenpAI/Core/GameModes/BP_GameState_ReinforcmentModel.BP_GameState_ReinforcmentModel_C|GetAI_model _asbp_game_state_reinforcment_model))
  (if (Utilities|Array|IsEmpty (Variables|Default|GetTagString))
    ;[1 1 1] Generate from Model
    (bind _returnvalue (Class|ReinforceModel|CreateEnemy (LocalVariables|GetReinforcmentModel)))
    (bind _output_get (Variables|Default|SetEnemyConfig _returnvalue))
    (Default|ApplyTags (LocalVariables|GetAIController) _output_get (Class|ReinforceModel|EnemytoIntArray (LocalVariables|GetReinforcmentModel) (Variables|Default|GetEnemyConfig)) false)
    (else
      ;[1 1 1] Use selected Tags
      (bind _output_get_2 (Variables|Default|SetEnemyConfig (Variables|Default|GetTagString)))
      (Default|ApplyTags (LocalVariables|GetAIController) _output_get_2 (Class|ReinforceModel|EnemytoIntArray (LocalVariables|GetReinforcmentModel) (Variables|Default|GetEnemyConfig)) true))))