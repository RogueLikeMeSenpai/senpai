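; BP_DoorSimple is a simple door actor that swings open when its Open event is called.
; Open plays a door sound in 2D and runs a timeline that scales a curve by an Angle variable to set the bottom pivot's relative yaw.
; BeginPlay caches the Senpai game mode and the game instance, though nothing else in the graph uses them.
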(event Custom|Open
  (Audio|PlaySound2D "/Game/SenpAI/Audio/Sounds/Environment/A_Door_open_Cue.A_Door_open_Cue" 1.0 1.0 0.0 0 0)
  (bind _doorrotation (Timeline|DoorRotation Play)
    (:Update
      (Transformation|SetRelativeRotation (Variables|Default|GetArch_Door_bottompivot) (Math|Rotator|MakeRotator 0.0 0.0 (* _doorrotation (Variables|Default|GetAngle))) false false))))

(event EventBeginPlay
  (bind _asbp_senpai_game_mode (Utilities|Casting|CastToBP_Senpai_GameMode (Game|GetGameMode)))
  (Variables|Default|SetgameMode _asbp_senpai_game_mode)
  (bind _asgame_instance_alex (Utilities|Casting|CastToGameInstanceAlex (Game|GetGameInstance)))
  (Variables|Default|SetgameInstance _asgame_instance_alex))

(event Collision|EventActorBeginOverlap
  (params (OtherActor :type Actor%20Object%20Reference)))

(event EventTick
  (params (DeltaSeconds :type Float%20%28single-precision%29)))

(fn ConstructionScript)