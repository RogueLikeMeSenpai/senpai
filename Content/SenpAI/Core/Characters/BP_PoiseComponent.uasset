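; Actor component that gives its owner a poise meter, staggering enemies when damage breaks it.
; It binds to the owner's any-damage event, subtracts raw damage from poise and regenerates poise over time on Tick, clamped to the maximum.
; At zero, poise resets to full and Stagger is called on the owner, which currently works only for BP_SimpleEnemy_Character.
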(event Custom|OnTakeAnyDamage
  (params (DamagedActor :type Actor%20Object%20Reference) (Damage :type Float%20%28single-precision%29) (DamageType :type Damage%20Type%20Object%20Reference) (InstigatedBy :type Controller%20Object%20Reference) (DamageCauser :type Actor%20Object%20Reference))
  (CallFunction|ApplyPoiseDamage Damage))

(event EventBeginPlay
  (Variables|Default|SetCurrentPoise (Variables|Default|GetMaxPoise))
  (EventDispatchers|BindEventtoOnTakeAnyDamage (Components|GetOwner) (delegate Custom|OnTakeAnyDamage)))

(event EventTick
  (params (DeltaSeconds :type Float%20%28single-precision%29))
  ;[1 1 1] Regenerate
  (Variables|Default|SetCurrentPoise (Math|Float|Clamp(Float) (+ (Variables|Default|GetCurrentPoise) (* DeltaSeconds (Variables|Default|GetRegenPerSecond))) 0.0 (Variables|Default|GetMaxPoise))))

(fn ApplyPoiseDamage
  (params (Damage :type Float%20%28double-precision%29))
  (bind _output_get (Variables|Default|SetCurrentPoise (Math|Float|Clamp(Float) (- (Variables|Default|GetCurrentPoise) Damage) 0.0 (Variables|Default|GetMaxPoise))))
  (if (<= _output_get 0.0)
    (Variables|Default|SetCurrentPoise (Variables|Default|GetMaxPoise))
    (bind _asbp_simple_enemy_character (Utilities|Casting|CastToBP_SimpleEnemy_Character (Components|GetOwner))) ; TODO: BaseCharacter
    (Default|Stagger _asbp_simple_enemy_character)))