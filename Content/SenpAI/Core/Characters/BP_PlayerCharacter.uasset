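; BP_PlayerCharacter is the player character, with switchable melee and ranged weapons, a health bar and death handling.
; SpawnWeapon replaces the current weapon actor and attaches it to the right hand socket; attacking plays a punch montage and calls the weapon's Attack if it can attack.
; HealthComponent events update the health bar widget and, on death, disable control and reload the current level after a short delay.
; BeginPlay also adds a pause menu widget to the viewport.
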(event OnDeath(HealthComponent)
  (params (DeadActor :type Actor%20Object%20Reference))
  ;[0 1 0.2039] Death
  (Variables|Default|SetIsDead true)
  (Development|PrintString "Game Over")
  (Pawn|Components|CharacterMovement|DisableMovement (Variables|Character|GetCharacterMovement))
  (Input|DisableInput 0)
  (Utilities|FlowControl|Delay 2.0)
  (bind _returnvalue (Game|GetCurrentLevelName true))
  (Game|OpenLevel(byName) (Utilities|String|StringToName _returnvalue)))

(event OnHealthChanged(HealthComponent)
  (params (Owner :type Actor%20Object%20Reference))
  (bind _healthcomponent (Variables|Default|GetHealthComponent))
  (bind _currenthealth (Variables|/Script/senpai.BaseHealthComponent|GetCurrentHealth _healthcomponent))
  ;[0 1 0.2039] Update Healthbar from HealthComponent
  (Default|UpdateHealth (Variables|Default|GetHealthBar_0) (/ _currenthealth (Variables|/Script/senpai.BaseHealthComponent|GetMaxHealth _healthcomponent)))
  (Development|PrintString (Utilities|String|ToString(Float) _currenthealth)))

(event EventBeginPlay
  ;[0 0.2131 1] Initialise Healthbar
  (bind _returnvalue (UserInterface|CreateWidget "/Game/SenpAI/Core/UI/WB_HealthBar.WB_HealthBar_C"))
  (UserInterface|Viewport|AddtoViewport _returnvalue 0)
  (Variables|Default|SetHealthBar_0 _returnvalue)
  ;[1 1 1] Spawn weapon on startup and attach it to hand socket
  (|CallParentFunction)
  (CallFunction|SpawnWeapon (Variables|Default|GetStartingWeaponType))
  ;[0.004774 0.1313 1] Pause Menu
  (bind _returnvalue_2 (UserInterface|CreateWidget "/Game/SenpAI/Core/UI/WB_Pause_Menu.WB_Pause_Menu_C"))
  (UserInterface|Viewport|AddtoViewport _returnvalue_2 0))

(event Input|ActionEvents|InputActionAttack
  (params (Key :type Key%20Structure :default "None"))
  (:Pressed
    (CallFunction|Attack 0.0)))

(event Input|ActionEvents|InputActionSwitchWeapon
  (params (Key :type Key%20Structure :default "None"))
  (:Pressed
    (if (== (Variables|Default|GetCurrentWeaponType) (Variables|Default|GetMelee%20Weapon%20Type))
      (CallFunction|SpawnWeapon (Variables|Default|GetRanged%20Weapon%20Type))
      (else
        (CallFunction|SpawnWeapon (Variables|Default|GetMelee%20Weapon%20Type))))))

(fn ConstructionScript
  (|CallParentFunction))

(fn Attack
  (params (Delay%20between%20Attack%20and%20Animation :type Float%20%28double-precision%29))
  (if (Variables|/Script/senpai.BaseWeapon|GetbCanAttack (Variables|Default|GetWeaponActor))
    (Animation|PlayAnimMontage "/Game/SenpAI/Characters/Mannequins/Animations/Quinn/Punching_Retargeted_Montage.Punching_Retargeted_Montage" 1.0 "None")
    (Class|BaseWeapon|Attack (Variables|Default|GetWeaponActor))))

(fn SpawnWeapon
  (params (Type :type Base%20Weapon%20Class%20Reference))
  (if (Utilities|IsValid (Variables|Default|GetWeaponActor))
    (Actor|DestroyActor (Variables|Default|GetWeaponActor)))
  (bind _returnvalue (Game|SpawnActorfromClass Type (Math|Conversions|ToTransform(Vector) (Transformation|GetActorLocation)) "AlwaysSpawn" 0 0))
  (Variables|Default|SetCurrentWeaponType Type)
  (Transformation|AttachComponentToComponent _returnvalue (Variables|Character|GetMesh) "HandSocket_r" "SnapToTarget" "KeepRelative" "KeepRelative" true)
  (Variables|Default|SetWeaponActor _returnvalue)
  (Variables|/Script/senpai.BaseWeapon|SetWeaponOwner _returnvalue self))