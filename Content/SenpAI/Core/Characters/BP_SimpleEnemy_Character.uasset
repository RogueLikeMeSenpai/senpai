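; Simple enemy character with health, stagger and stamina components, socket-attached weapons, armor, state text and walk/run speeds.
; Component events update the health-bar widget, knock the enemy down on full stagger, and on death play an animation and scatter BP_Soul pickups on nearby navmesh.
; Attacks spend stamina and return montage duration from per-weapon configs.
; Capsule hits at near-zero speed briefly signal AIC_SimpleEnemy that it is stuck on an edge.
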(event OnDeath(HealthComponent)
  (params (DeadActor :type Actor%20Object%20Reference))
  (Variables|Default|SetshouldUIUpdate false)
  (Components|Animation|PlayAnimation (Variables|Character|GetMesh) "/Game/SenpAI/Characters/Assyrian/A_Assyrian_StandingDeathForward01.A_Assyrian_StandingDeathForward01" false)
  (for _index (range 1 (Variables|Default|Getsouls))
    (bind (_randomlocation _returnvalue) (Class|NavigationSystemV1|GetRandomLocationinNavigableRadius (Transformation|GetActorLocation) 1e+02 0 0))
    (if _returnvalue
      (Game|SpawnActorfromClass "/Game/SenpAI/Core/Environment/BP_Soul.BP_Soul_C" (Math|Transform|MakeTransform (+ _randomlocation "0,0,100.000000") "0, 0, 0" "1.000000,1.000000,1.000000") "Undefined" 0 0)
      (else
        (Game|SpawnActorfromClass "/Game/SenpAI/Core/Environment/BP_Soul.BP_Soul_C" (Math|Transform|MakeTransform (Transformation|GetActorLocation (Game|GetPlayerCharacter 0)) "0, 0, 0" "1.000000,1.000000,1.000000") "Undefined" 0 0)))))

(event OnHealthChanged(HealthComponent)
  (params (Owner :type Actor%20Object%20Reference))
  (bind _healthcomponent (Variables|Default|GetHealthComponent))
  ;[0 1 0.2039] Update Healthbar from HealthComponent
  (bind _aswb_health_bar_enemy (Utilities|Casting|CastToWB_HealthBar_Enemy (UserInterface|GetWidget (Variables|Default|GetBP_EnemyHealthBar))))
  (Default|UpdateHealth _aswb_health_bar_enemy (/ (Variables|/Script/senpai.BaseHealthComponent|GetCurrentHealth _healthcomponent) (Variables|/Script/senpai.BaseHealthComponent|GetMaxHealth _healthcomponent))))

(event OnComponentHit(CapsuleComponent)
  (params (HitComponent :type Primitive%20Component%20Object%20Reference) (OtherActor :type Actor%20Object%20Reference) (OtherComp :type Primitive%20Component%20Object%20Reference) (NormalImpulse :type Vector :default "0, 0, 0") (Hit :type Hit%20Result%20Structure%20%28by%20ref%29))
  (bind (_bblockinghit _binitialoverlap _time _distance _location _impactpoint _normal) (Collision|BreakHitResult Hit))
  ;[1 1 1] Detect if Stuck in Wall
  (if (< (Math|Vector|VectorLength (Variables|/Script/Engine.MovementComponent|GetVelocity (Variables|Character|GetCharacterMovement))) 12.0)
    (bind _asaic_simple_enemy (Utilities|Casting|CastToAIC_SimpleEnemy (Pawn|GetController)))
    (Default|BeginonEdge _asaic_simple_enemy _location _normal)
    (Utilities|FlowControl|Delay 0.2)
    (Default|EndonEdge _asaic_simple_enemy)))

(event OnFullStagger(StaggerComponent)
  (params (StaggeredActor :type Actor%20Object%20Reference))
  (bind _mesh (Variables|Character|GetMesh))
  (bind _returnvalue (Components|SkeletalMesh|GetAnimInstance _mesh))
  (Animation|Montage|MontageStop _returnvalue 0.0 (Animation|Montage|GetCurrentActiveMontage _returnvalue))
  (Animation|PlayAnimMontage "/Game/Developers/Christian/Assyrian_KnockDown.Assyrian_KnockDown" 1.0 "None")
  (Pawn|Components|CharacterMovement|DisableMovement (Variables|Character|GetCharacterMovement))
  (Development|PrintString "FULLY STAGGERED"))

(event OnStaggerReset(StaggerComponent)
  (params (StaggeredActor :type Actor%20Object%20Reference))
  (Pawn|Components|CharacterMovement|SetMovementMode (Variables|Character|GetCharacterMovement) "MOVE_Walking" 0)
  (Development|PrintString "STAGGER RESET"))

(event Custom|Stagger)

(event Custom|Unstagger)

(event EventBeginPlay)

(event Collision|EventActorBeginOverlap
  (params (OtherActor :type Actor%20Object%20Reference)))

(event EventTick
  (params (DeltaSeconds :type Float%20%28single-precision%29))
  (bind _stagger_component (Variables|Default|GetStagger%20Component))
  (|CallParentFunction DeltaSeconds)
  (if (Variables|Default|GetshouldUIUpdate)
    (bind _aswb_health_bar_enemy (Utilities|Casting|CastToWB_HealthBar_Enemy (UserInterface|GetWidget (Variables|Default|GetBP_EnemyHealthBar))))
    (Default|UpdateStaggerUI _aswb_health_bar_enemy (/ (Variables|/Script/senpai.BaseStaggerComponent|GetCurrentStaggerValue _stagger_component) (Variables|/Script/senpai.BaseStaggerComponent|GetMaxStaggerValue _stagger_component)))))

(fn ConstructionScript)

(fn SpawnWeapon
  (params (WeaponClass :type Base%20Weapon%20Class%20Reference))
  (bind _returnvalue (Game|SpawnActorfromClass WeaponClass (Transformation|GetActorTransform) "Undefined" 0 0))
  (bind _output_get (Variables|Default|SetWeapon _returnvalue))
  (Transformation|AttachComponentToComponent _output_get (Variables|Character|GetMesh) (.Value (Utilities|Map|Find (Variables|Default|GetweaponSocketConfig) (Variables|/Script/senpai.WeaponDataAsset|GetHandSocket (.Value (Utilities|Map|Find (Variables|Default|GetweaponConfigs) WeaponClass))))) "SnapToTarget" "KeepRelative" "KeepRelative" true)
  (Variables|/Script/senpai.BaseWeapon|SetWeaponOwner (Variables|Default|GetWeapon) self)
  (return (Variables|Default|GetWeapon)))

(fn ChangeState
  (params (State :type Enum_SimpleEnemyState%20Enum :default "NewEnumerator0"))
  (switch Utilities|FlowControl|Switch|SwitchonEnum_SimpleEnemyState State
    (:NewEnumerator0
      (Rendering|Components|TextRender|SetText (Variables|Default|GetTextState) (LocalVariables|GetTextRoaming)))
    (:NewEnumerator2
      (Rendering|Components|TextRender|SetText (Variables|Default|GetTextState) (LocalVariables|GetTextEngaged)))
    (:NewEnumerator1
      (Rendering|Components|TextRender|SetText (Variables|Default|GetTextState) (LocalVariables|GetTextSearching)))))

(fn PrimaryAttack
  (bind _weaponconfigs (Variables|Default|GetweaponConfigs))
  (bind _weapon (Variables|Default|GetWeapon))
  (bind _returnvalue (Utilities|GetClass _weapon))
  (bind _value (Utilities|Map|Find _weaponconfigs _returnvalue))
  (bind _primaryattackplayrate (Variables|/Script/senpai.WeaponDataAsset|GetPrimaryAttackPlayRate _value))
  (bind _returnvalue_2 (Class|BaseStaminaComponent|UseStamina (Variables|Default|GetStamina%20Component) (Variables|/Script/senpai.WeaponDataAsset|GetPrimaryStaminaCost _value)))
  (if _returnvalue_2
    (bind _returnvalue_3 (Animation|PlayAnimMontage (Variables|/Script/senpai.WeaponDataAsset|GetPrimaryAttackMontage _value) _primaryattackplayrate "None"))
    (return (/ _returnvalue_3 _primaryattackplayrate) true)
    (else
      (return 0.0 false))))

(fn SpawnArmor
  (params (armorClass :type BP%20Item%20Boost%20Class%20Reference))
  (bind _returnvalue (Game|SpawnActorfromClass armorClass (Transformation|GetActorTransform) "Undefined" 0 self 0))
  (Transformation|AttachActorToActor _returnvalue self "None" "KeepRelative" "KeepRelative" "KeepRelative" true))

(fn SecondaryAttack
  (bind _weaponconfigs (Variables|Default|GetweaponConfigs))
  (bind _weapon (Variables|Default|GetWeapon))
  (bind _returnvalue (Utilities|GetClass _weapon))
  (bind _value (Utilities|Map|Find _weaponconfigs _returnvalue))
  (bind _secondaryattackplayrate (Variables|/Script/senpai.WeaponDataAsset|GetSecondaryAttackPlayRate _value))
  (bind _returnvalue_2 (Class|BaseStaminaComponent|UseStamina (Variables|Default|GetStamina%20Component) (Variables|/Script/senpai.WeaponDataAsset|GetSecondaryStaminaCost _value)))
  (if _returnvalue_2
    (bind _returnvalue_3 (Animation|PlayAnimMontage (Variables|/Script/senpai.WeaponDataAsset|GetSecondaryAttackMontage _value) _secondaryattackplayrate "None"))
    (return (/ _returnvalue_3 _secondaryattackplayrate) true)
    (else
      (return 0.0 false))))

(fn ChangeWalkingMode
  (params (movementMode :type Enum_WalkingMode%20Enum :default "NewEnumerator0"))
  (switch Utilities|FlowControl|Switch|SwitchonEnum_WalkingMode movementMode
    (:NewEnumerator0
      (Variables|/Script/Engine.CharacterMovementComponent|SetMaxWalkSpeed (Variables|Character|GetCharacterMovement) (Variables|Default|GetwalkingSpeed)))
    (:NewEnumerator1
      (Variables|/Script/Engine.CharacterMovementComponent|SetMaxWalkSpeed (Variables|Character|GetCharacterMovement) (Variables|Default|GetrunningSpeed)))))