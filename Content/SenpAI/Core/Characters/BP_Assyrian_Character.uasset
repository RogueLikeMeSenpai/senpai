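; Assyrian enemy character Blueprint that supplies melee and ranged attack animations and death cleanup on top of its parent class.
; PlayMeleeAttack and PlayRangedAttack play montages for a standing horizontal melee swing and a mirrored bow shot.
; When the health component signals death, it disables actor collision and destroys the enemy health bar component.
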(event OnDeath(HealthComponent)
  (params (DeadActor :type Actor%20Object%20Reference))
  (Collision|SetActorEnableCollision false)
  (Components|DestroyComponent (Variables|Default|GetBP_EnemyHealthBar)))

(event EventBeginPlay
  (|CallParentFunction))

(event Collision|EventActorBeginOverlap
  (params (OtherActor :type Actor%20Object%20Reference)))

(event EventTick
  (params (DeltaSeconds :type Float%20%28single-precision%29)))

(fn ConstructionScript
  (|CallParentFunction))

(fn PlayMeleeAttack
  (Animation|PlayAnimMontage "/Game/SenpAI/Characters/Assyrian/AM_Assyrian_StandingMeleeAttackHorizontal.AM_Assyrian_StandingMeleeAttackHorizontal" 1.0 "None"))

(fn PlayRangedAttack
  (Animation|PlayAnimMontage "/Game/SenpAI/Characters/Assyrian/AM_Assyrian_ShootingArrow_Mirrored.AM_Assyrian_ShootingArrow_Mirrored" 1.0 "None"))