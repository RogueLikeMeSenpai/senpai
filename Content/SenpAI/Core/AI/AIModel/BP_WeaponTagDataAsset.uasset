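; BP_WeaponTagDataAsset is an AI tag data asset that equips an AI character with a weapon.
; When its value converts to true, Apply sets a blackboard key, spawns the configured weapon class on the character, binds its events to the controller and assigns the controller's attack strategies.
; The key is only ever set to true, a noted workaround until hammer behavior is included.
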(fn Apply
  (params (aiController :type AIC%20Simple%20Enemy%20Object%20Reference) (value :type Integer) (character :type BP%20Simple%20Enemy%20Character%20Object%20Reference))
  ;[1 1 1] Only setting blackboard key to true, because of workaround until hammer behavior is included
  (if (Math|Conversions|ToBoolean(Integer) value)
    (AI|Components|Blackboard|SetValueasBool (AI|GetBlackboard aiController) (Variables|Default|GetblackboardKey) true)
    (bind _weapon (Default|SpawnWeapon character (Variables|Default|GetweaponClass)))
    (Default|BindWeaponEvents aiController _weapon)
    (Variables|/Game/SenpAI/Core/AI/AIC_SimpleEnemy.AIC_SimpleEnemy_C|SetattackStrategies aiController (Variables|Default|GetattackStrategies))))