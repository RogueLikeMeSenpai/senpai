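; Behavior tag data asset in the SenpAI AI model that applies a value to an AI controller to toggle a behavior and choose its attack strategy.
; Apply writes the value as a bool to the configured blackboard key.
; When true, it looks up its AttackStrategy in the controller's AttackStrategies map and injects that behavior tree as the dynamic subtree under the EngagedBehavior tag.
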(fn Apply
  (params (aiController :type AIC%20Simple%20Enemy%20Object%20Reference) (value :type Integer) (character :type BP%20Simple%20Enemy%20Character%20Object%20Reference))
  (AI|Components|Blackboard|SetValueasBool (AI|GetBlackboard aiController) (Variables|Default|GetblackboardKey) (Math|Conversions|ToBoolean(Integer) value))
  (if (Math|Conversions|ToBoolean(Integer) value)
    (bind _asbehavior_tree_component (Utilities|Casting|CastToBehaviorTreeComponent (Variables|/Script/AIModule.AIController|GetBrainComponent aiController)))
    (Class|BehaviorTreeComponent|SetDynamicSubtree _asbehavior_tree_component "(TagName=\"EngagedBehavior\")" (.Value (Utilities|Map|Find (Variables|/Game/SenpAI/Core/AI/AIC_SimpleEnemy.AIC_SimpleEnemy_C|GetattackStrategies aiController) (Variables|Default|GetattackStrategy))))))