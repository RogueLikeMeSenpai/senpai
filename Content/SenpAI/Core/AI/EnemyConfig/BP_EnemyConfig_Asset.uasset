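; BP_EnemyConfig_Asset holds the EnemyConfigs array for the AI system and provides lookups into it by Id.
; GetConfigStrings loops over the array and returns a list of unique config Ids.
; GetEnemyConfig searches the array linearly and stops at the first entry whose Id matches, returning that config.
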(fn GetConfigStrings
  (for _array_element (Variables|Default|GetEnemyConfigs)
    (Utilities|Array|AddUnique (LocalVariables|GetConfigIds) (.id _array_element)))
  (return (LocalVariables|GetConfigIds)))

(fn GetEnemyConfig
  (params (id :type String))
  (bind _array_element (Utilities|Array|ForEachLoopwithBreak (Variables|Default|GetEnemyConfigs) :!label _label)
    (:LoopBody
      (if (Utilities|Enum|Equal(Enum) (.Id (Utilities|Struct|BreakStructure_EnemyConfig _array_element)) id)
        (LocalVariables|SetEnemyConfig _array_element)
        (goto _label Break)))
    (:Completed
      (return (LocalVariables|GetEnemyConfig)))))