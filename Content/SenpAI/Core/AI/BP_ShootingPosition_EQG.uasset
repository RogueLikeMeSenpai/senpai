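; EQS generator that produces candidate shooting positions for AI around player character 0.
; It samples points on a ring of Radius around the player at 20-degree steps, ignoring the supplied context locations.
; Each point runs a debug-drawn box multi-trace to the player on the Visibility channel, and only points whose trace reports no blocking hit become query items.
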(fn DoItemGeneration
  (params (ContextLocations :type Array%20of%20Vectors))
  (bind _returnvalue (Game|GetPlayerCharacter 0))
  (bind _returnvalue_2 (Transformation|GetActorLocation _returnvalue))
  (for _index (range 0 18)
    (bind _returnvalue_3 (Class|KismetSystemLibrary|BoxTraceMulti (+ (* (Math|Vector|RotateVector "1.000000, 0, 0" (Math|Rotator|MakeRotator 0.0 0.0 (* _index 2e+01))) (Variables|Default|GetRadius)) _returnvalue_2) _returnvalue_2 "40.000000,40.000000,40.000000" "0, 0,0.000000" "TraceTypeQuery1" false 0 "ForDuration" true))
    (if (not _returnvalue_3)
      (Class|EnvQueryGeneratorBlueprintBase|AddGeneratedVector (+ (* (Math|Vector|RotateVector "1.000000, 0, 0" (Math|Rotator|MakeRotator 0.0 0.0 (* _index 2e+01))) (Variables|Default|GetRadius)) _returnvalue_2))))
  (return))