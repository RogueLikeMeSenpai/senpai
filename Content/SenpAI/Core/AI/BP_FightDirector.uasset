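; Fight director actor that picks which simple enemy attacks, keeping a fighting grade per enemy, seeded randomly at BeginPlay.
; TriggerAttack scales each grade by how opposed the enemy's and player's forward vectors are, switches the top enemy's AI controller to attacking, then re-randomizes its grade.
; The looping timer and debug widget code are disconnected, so TriggerAttack needs an outside caller.
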(event Custom|TriggerAttack
  (CallFunction|RecalculateFightingGrades)
  ;[1 1 1] Trigger Attack on highest Graded Enemy
  (bind _loc_highestgradedenemy1 (CallFunction|FindHighestGrade))
  (bind _asaic_simple_enemy (Utilities|Casting|CastToAIC_SimpleEnemy (AI|GetAIController _loc_highestgradedenemy1)))
  (Default|ChangeStatetoAttacking _asaic_simple_enemy)
  ;[1 1 1] Reassign Grade of Attacking Enemy to a random number
  (Utilities|Map|Add (Variables|Default|GetEnemyGrading) _loc_highestgradedenemy1 (Math|Random|RandomFloatinRange 1.0 5.0)))

(event EventBeginPlay
  ;[1 1 1] Initialize with Enemy Characters
  (bind _outactors (Actor|GetAllActorsOfClass "/Game/SenpAI/Core/Characters/BP_SimpleEnemy_Character.BP_SimpleEnemy_Character_C"))
  (for _array_element _outactors
    (bind _asbp_simple_enemy_character (Utilities|Casting|CastToBP_SimpleEnemy_Character _array_element))
    (Utilities|Array|Add (Variables|Default|GetEnemyList) _asbp_simple_enemy_character)
    (CallFunction|InitializeFightingGrade _asbp_simple_enemy_character)))

(event Collision|EventActorBeginOverlap
  (params (OtherActor :type Actor%20Object%20Reference)))

(event EventTick
  (params (DeltaSeconds :type Float%20%28single-precision%29)))

(fn ConstructionScript)

(fn FindHighestGrade
  (bind _keys (Utilities|Map|Keys (Variables|Default|GetEnemyGrading)))
  (for _array_element _keys
    (if (> (.Value (Utilities|Map|Find (Variables|Default|GetEnemyGrading) _array_element)) (LocalVariables|GetLoc_HighestValue))
      (Utilities|FlowControl|Sequence
        (:then_0
          (LocalVariables|SetLoc_HighestValue (.Value (Utilities|Map|Find (Variables|Default|GetEnemyGrading) _array_element))))
        (:then_1
          (LocalVariables|SetLoc_HighestGradedEnemy _array_element)))))
  (return (LocalVariables|GetLoc_HighestValue) (LocalVariables|GetLoc_HighestGradedEnemy)))

(fn InitializeFightingGrade
  (params (EnemyInstance :type BP%20Simple%20Enemy%20Character%20Object%20Reference%20%28by%20ref%29))
  ;[1 1 1] Assign random fighting grade
  (Utilities|Map|Add (Variables|Default|GetEnemyGrading) EnemyInstance (Math|Random|RandomFloatinRange 1.0 5.0)))

(fn UpdateDebugWidget
  (params (EnemyInstance :type BP%20Simple%20Enemy%20Character%20Object%20Reference))
  (Variables|/Game/SenpAI/Core/AI/WBP_DebugSimpleEnemy.WBP_DebugSimpleEnemy_C|SetFightingGrade (.Value (Utilities|Map|Find (Variables|Default|GetEnemyWidgets) EnemyInstance)) (.Value (Utilities|Map|Find (Variables|Default|GetEnemyGrading) EnemyInstance))))

(fn RecalculateFightingGrades
  (for _array_element (Variables|Default|GetEnemyList)
    (CallFunction|GradebyPosition _array_element)))

(fn GradebyPosition
  (params (EnemyInstance :type BP%20Simple%20Enemy%20Character%20Object%20Reference))
  (bind _enemygrading (Variables|Default|GetEnemyGrading))
  (Utilities|Map|Add _enemygrading EnemyInstance (* (.Value (Utilities|Map|Find _enemygrading EnemyInstance)) (+ (Math|Float|NormalizetoRange (* (Math|Vector|DotProduct (Transformation|GetActorForwardVector EnemyInstance) (Transformation|GetActorForwardVector (Game|GetPlayerCharacter 0))) -1.0) -1.0 1.0) 0.5))))