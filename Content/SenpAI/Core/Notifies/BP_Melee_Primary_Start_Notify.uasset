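; An animation notify that fires a character's primary melee attack at a point in an animation.
; It casts the mesh owner to the player character, or failing that to the simple enemy character, and calls UsePrimaryAttack on that character's weapon.
; The player branch also prints a "Start Trace" debug string.
; Its display name reads "End Melee Primary" despite the Start asset name.
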(fn GetNotifyName
  (return "End Melee Primary"))

(fn ReceivedNotify
  (params (MeshComp :type Skeletal%20Mesh%20Component%20Object%20Reference) (Animation :type Anim%20Sequence%20Base%20Object%20Reference) (EventReference :type Anim%20Notify%20Event%20Reference%20Structure%20%28by%20ref%29))
  (bind _returnvalue (Components|GetOwner MeshComp))
  (bind _asbp_player_character (Utilities|Casting|CastToBP_PlayerCharacter _returnvalue)
    (:then
      (Class|BaseWeapon|UsePrimaryAttack (Variables|/Game/SenpAI/Core/Characters/BP_PlayerCharacter.BP_PlayerCharacter_C|GetWeaponActor _asbp_player_character))
      (Development|PrintString "Start Trace"))
    (:CastFailed
      (bind _asbp_simple_enemy_character (Utilities|Casting|CastToBP_SimpleEnemy_Character _returnvalue))
      (Class|BaseWeapon|UsePrimaryAttack (Variables|/Game/SenpAI/Core/Characters/BP_SimpleEnemy_Character.BP_SimpleEnemy_Character_C|GetWeapon _asbp_simple_enemy_character))))
  (return false))