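; Base hammer weapon Blueprint that gives its owner a secondary area-of-effect melee attack.
; Ending the attack sets the owning Character to Walking, then applies full radial melee damage around the Box's center of mass, sparing the owner.
; A scaled-up attack effect spawns at the same point.
; Starting the attack only casts the owner, as the DisableMovement call is disconnected.
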(event EventUseSecondaryAttack
  (bind _ascharacter (Utilities|Casting|CastToCharacter (Variables|Default|GetWeaponOwner))))

(event EventEndSecondaryAttack
  (bind _weaponowner (Variables|Default|GetWeaponOwner))
  (bind _box (Variables|Default|GetBox))
  (bind _returnvalue (Physics|GetCenterOfMass _box "None"))
  (bind _ascharacter (Utilities|Casting|CastToCharacter _weaponowner))
  (Pawn|Components|CharacterMovement|SetMovementMode (Variables|/Script/Engine.Character|GetCharacterMovement _ascharacter) "MOVE_Walking" 0)
  (Game|Damage|ApplyRadialDamage (Variables|Default|GetSecondaryBaseDamage) _returnvalue 3e+02 "/Game/SenpAI/Core/Weapons/BP_MeleeDamageType.BP_MeleeDamageType_C" (Utilities|Array|MakeArray _weaponowner) _weaponowner 0 true "ECC_Visibility")
  (Niagara|SpawnSystematLocation (Variables|Default|GetAttackEffect) _returnvalue "0, 0, 0" "4.000000,4.000000,4.000000"))

(fn ConstructionScript
  (|CallParentFunction))