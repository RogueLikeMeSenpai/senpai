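; Base secondary weapon projectile that damages the first valid actor it overlaps, then destroys itself.
; On overlap it casts its owner to BaseWeapon and ignores that weapon's owner.
; For other actors it calls the DamageDealt dispatcher, applies its Damage with the weapon's owner as causer, spawns the particle effect and stops movement.
; The environment-hit message and delayed destroy are disconnected and never run.
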(event Collision|EventActorBeginOverlap
  (params (OtherActor :type Actor%20Object%20Reference))
  (bind _damage (Variables|Default|Getdamage))
  ;[1 1 1] Deal Damage on Overlapping with an actor
  (bind _asbase_weapon (Utilities|Casting|CastToBaseWeapon (Components|GetOwner)))
  (if (not (== OtherActor (Variables|/Script/senpai.BaseWeapon|GetWeaponOwner _asbase_weapon)))
    (bind _asactor (Utilities|Casting|CastToActor OtherActor))
    (Default|CallDamageDealt _damage _asactor :!pinned true) ; Get damage from ProjectileOwner
    (Game|Damage|ApplyDamage OtherActor _damage 0 (Variables|/Script/senpai.BaseWeapon|GetWeaponOwner _asbase_weapon) (Variables|Default|GetDamageType))
    (Niagara|SpawnSystematLocation (Variables|Default|GetParticleEffect) (Transformation|GetActorLocation))
    (Components|Movement|StopMovementImmediately (Variables|Default|GetProjectileMovement))
    (Actor|DestroyActor)))

(fn ConstructionScript)