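; Base projectile actor that damages whatever actor it overlaps, ignoring its own owner.
; On overlap it fires the DamageDealt dispatcher and applies a hard-coded damage amount, crediting the owner as damage causer.
; It then prints a debug message, spawns its particle effect at its location and destroys itself.
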(event Collision|EventActorBeginOverlap
  (params (OtherActor :type Actor%20Object%20Reference))
  (bind _returnvalue (Components|GetOwner))
  ;[1 1 1] Deal Damage on Overlapping with an actor
  (if (not (== OtherActor _returnvalue))
    (Default|CallDamageDealt 1e+02 OtherActor) ; Get damage from ProjectileOwner
    (Game|Damage|ApplyDamage OtherActor 1e+02 0 _returnvalue (Variables|Default|GetDamageType))
    (Development|PrintString "Projectile dies")
    (Niagara|SpawnSystematLocation (Variables|Default|GetParticleEffect) (Transformation|GetActorLocation))
    (Actor|DestroyActor)))

(fn ConstructionScript)