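; Base ranged weapon Blueprint that extends its parent weapon's attack by firing a projectile.
; When Attack is called and CanAttack is true, it spawns the Projectile class at the mesh's ArrowSpawnSocket, always ignoring collision.
; The projectile takes its rotation from the attach parent actor rather than the socket, then the parent attack runs and a debug string prints.
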(event EventAttack
  ;[1 1 1] Spawn a projectile when attack function is called
  (if (Variables|Default|GetbCanAttack)
    (Game|SpawnActorfromClass (Variables|Default|GetProjectile) (Math|Transform|MakeTransform (Transformation|GetSocketLocation (Variables|Default|GetMeshComp) "ArrowSpawnSocket") (Transformation|GetActorRotation (Actor|GetAttachParentActor))) "AlwaysSpawn" 0 0)
    (|CallParentFunction)
    (Development|PrintString "Peng!")))

(fn ConstructionScript)