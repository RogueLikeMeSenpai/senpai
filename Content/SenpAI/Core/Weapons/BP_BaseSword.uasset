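; BP_BaseSword is a base sword weapon Blueprint that defines how a secondary attack opens and closes its damage window.
; Starting the secondary attack turns on tracing, sets the current damage to the secondary base value and casts the weapon owner to Character.
; Ending it stops tracing and clears the list of characters already hit.
; A DisableMovement call on the owner's movement is left disconnected.
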(event EventUseSecondaryAttack
  (Variables|Default|SetIs%20Tracing true)
  (Variables|Default|SetCurrentDamage (Variables|Default|GetSecondaryBaseDamage))
  (bind _ascharacter (Utilities|Casting|CastToCharacter (Variables|Default|GetWeaponOwner))))

(event EventEndSecondaryAttack
  (Variables|Default|SetIs%20Tracing false)
  (Utilities|Array|Clear (Variables|Default|GetCharacters%20Hit)))

(fn ConstructionScript
  (|CallParentFunction))