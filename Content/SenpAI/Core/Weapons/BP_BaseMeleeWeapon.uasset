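; Base melee weapon Blueprint that damages pawns it overlaps during a primary attack.
; A primary attack plays effects and opens a swing window lasting the primary cooldown, then resets the swing and hit flags.
; While swinging, actor overlap applies base damage to the first pawn other than the owner and triggers a damage-dealt notification, allowing one hit per swing.
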(event Collision|EventActorBeginOverlap
  (params (OtherActor :type Actor%20Object%20Reference))
  ;[1 1 1] Damage on Overlap
  (if (Variables|Default|GetIs%20Swinging)
    (if (not (Variables|Default|GetDid%20Current%20Attack%20Hit))
      (bind _aspawn (Utilities|Casting|CastToPawn OtherActor))
      (if (== _aspawn (Variables|Default|GetWeaponOwner))
        (Development|PrintString "Overlapped with owner" true true "(R=1.000000,G=0.000000,B=0.231619,A=1.000000)")
        (else
          (Variables|Default|SetDid%20Current%20Attack%20Hit true)
          (bind _returnvalue (Game|Damage|ApplyDamage _aspawn (Variables|Default|GetPrimaryBaseDamage) 0 (Variables|Default|GetWeaponOwner) (Variables|Default|GetDamageType)))
          (Class|BaseWeapon|TriggerDamageDealt _returnvalue _aspawn))))))

(event EventUsePrimaryAttack
  ;[1 1 1] Start Attack
  (if (Variables|Default|GetbCanUsePrimaryAttack)
    (Class|BaseWeapon|PlayAttackEffects)
    (Variables|Default|SetIs%20Swinging true)
    (Utilities|FlowControl|Delay (Variables|Default|GetPrimaryCooldown))
    (Variables|Default|SetIs%20Swinging false)
    (Variables|Default|SetDid%20Current%20Attack%20Hit false)))

(fn ConstructionScript)