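; Health boost item that raises the max health of the character it is attached to and visually armors it.
; On BeginPlay it multiplies the owner's HealthComponent max health by BoostFactor and refills current health to the new maximum.
; It then loops over the ArmorConfig data table, spawning a static mesh per row and snapping it to that row's socket on the owner's mesh.
; Older hardcoded helmet and chest attachment nodes remain unconnected.
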(event EventBeginPlay
  (bind _attachedto (Variables|Default|GetAttachedTo))
  (bind _healthcomponent (Variables|/Game/SenpAI/Core/Characters/BP_BaseCharacter.BP_BaseCharacter_C|GetHealthComponent _attachedto))
  (bind _output_get (Variables|/Script/senpai.BaseHealthComponent|SetMaxHealth _healthcomponent (* (Variables|/Script/senpai.BaseHealthComponent|GetMaxHealth _healthcomponent) (Variables|Default|GetboostFactor))))
  (Variables|/Script/senpai.BaseHealthComponent|SetCurrentHealth _healthcomponent _output_get)
  (bind _outrownames (DataTable|GetDataTableRowNames (Variables|Default|GetArmorConfig)))
  (for _array_element _outrownames
    ;[1 1 1] Attach Armor Piece
    (bind _returnvalue (Utilities|GetDataTableRow (Variables|Default|GetArmorConfig) _array_element)
      (:then
        (bind _returnvalue_2 (AddComponent|AddStaticMeshComponent (Variables|Default|GetAttachedTo) false))
        (Components|StaticMesh|SetStaticMesh _returnvalue_2 (.StaticMesh (Utilities|Struct|BreakStructure_Equipment _returnvalue)))
        (Transformation|AttachComponentToComponent _returnvalue_2 (Variables|/Script/Engine.Character|GetMesh (Variables|Default|GetAttachedTo)) (.Socket (Utilities|Struct|BreakStructure_Equipment _returnvalue)) "SnapToTarget" "SnapToTarget" "SnapToTarget" true)))))

(event Collision|EventActorBeginOverlap
  (params (OtherActor :type Actor%20Object%20Reference)))

(event EventTick
  (params (DeltaSeconds :type Float%20%28single-precision%29)))

(fn ConstructionScript
  (|CallParentFunction))