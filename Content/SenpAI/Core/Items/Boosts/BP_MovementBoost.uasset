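; BP_MovementBoost is a boost item that speeds up the character it is attached to.
; On BeginPlay it multiplies the AttachedTo character's Max Walk Speed and Max Acceleration on its CharacterMovement component by BoostFactor.
; The change is applied once, and this Blueprint has no logic to revert it.
; The construction script only calls its parent.
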(event EventBeginPlay
  (bind _attachedto (Variables|Default|GetAttachedTo))
  (bind _attachedto_2 (Variables|Default|GetAttachedTo))
  (bind _charactermovement (Variables|/Script/Engine.Character|GetCharacterMovement _attachedto_2))
  (bind _charactermovement_2 (Variables|/Script/Engine.Character|GetCharacterMovement _attachedto))
  (Utilities|FlowControl|Sequence
    (:then_0
      ;[1 1 1] Increase Max Walk Speed
      (Variables|/Script/Engine.CharacterMovementComponent|SetMaxWalkSpeed _charactermovement_2 (* (Variables|Default|GetboostFactor) (Variables|/Script/Engine.CharacterMovementComponent|GetMaxWalkSpeed _charactermovement_2))))
    (:then_1
      ;[1 1 1] Increase Max Acceleration
      (Variables|/Script/Engine.CharacterMovementComponent|SetMaxAcceleration _charactermovement (* (Variables|Default|GetboostFactor) (Variables|/Script/Engine.CharacterMovementComponent|GetMaxAcceleration _charactermovement))))))

(event Collision|EventActorBeginOverlap
  (params (OtherActor :type Actor%20Object%20Reference)))

(event EventTick
  (params (DeltaSeconds :type Float%20%28single-precision%29)))

(fn ConstructionScript
  (|CallParentFunction))