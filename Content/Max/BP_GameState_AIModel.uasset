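; Game state Blueprint that bridges an AI model to enemy creation by decoding an enemy string into melee and ranged flags.
; ParseEnemyAIString splits the comma-separated EnemyString into an AI model output struct.
; BeginPlay and CreateEnemy both call a placeholder AIModel function, then parse EnemyString; BeginPlay prints the flags, CreateEnemy returns them.
; A comment marks the call for replacement by C++, and GiveReward is an empty stub.
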(event EventBeginPlay
  (Class|TestActorComponentAIModel|MySuperDuperCoolFunction (Variables|Default|GetAIModel))
  (bind _aimodeloutput (CallFunction|ParseEnemyAIString (Variables|Default|GetEnemyString)))
  (Development|PrintString (Utilities|String|Append "Melee: " (Utilities|String|ToString(Boolean) (.Melee (Utilities|Struct|BreakBPStructure_AIModelOutput _aimodeloutput))) ", Ranged: " (Utilities|String|ToString(Boolean) (.Ranged (Utilities|Struct|BreakBPStructure_AIModelOutput _aimodeloutput))))))

(event EventTick
  (params (DeltaSeconds :type Float%20%28single-precision%29)))

(fn ConstructionScript)

(fn ParseEnemyAIString
  (params (EnemyAIString :type String))
  (LocalVariables|SetEnemyStringArray (Utilities|String|ParseIntoArray EnemyAIString ","))
  (return (Utilities|Struct|MakeBPStructure_AIModelOutput (Math|Conversions|ToBoolean(Integer) (Math|Conversions|ToInteger(Byte) (Utilities|Array|Get(acopy) (LocalVariables|GetEnemyStringArray)))) (Math|Conversions|ToBoolean(Integer) (Math|Conversions|ToInteger(Byte) (Utilities|Array|Get(acopy) (LocalVariables|GetEnemyStringArray) 1))))))

(fn CreateEnemy
  ;[1 1 1] This will be replaced by C++ function call which returns the enemy String
  (Class|TestActorComponentAIModel|MySuperDuperCoolFunction (Variables|Default|GetAIModel))
  (bind _aimodeloutput (CallFunction|ParseEnemyAIString (Variables|Default|GetEnemyString)))
  (return _aimodeloutput))

(fn GiveReward)